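; BP_CameraPawn is a camera pawn that pans horizontally and zooms with a spring arm.
; Pan input axes shift a target location along world X and Y, while the zoom axis adjusts a target arm length clamped between minimum and maximum zoom.
; Each Tick lerps the root position and arm length toward those targets by fixed alphas, giving smooth but frame-rate-dependent easing.
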(event EventTick
  (params (DeltaSeconds :type Float%20%28single-precision%29))
  (bind _springarm (Variables|Default|GetSpringArm))
  (Transformation|SetWorldLocation (Variables|Default|GetDefaultSceneRoot) (Math|Vector|Lerp(Vector) (Transformation|GetWorldLocation (Variables|Default|GetDefaultSceneRoot)) (Variables|Camera|GetTargetToPan) 0.075) false false)
  (Variables|/Script/Engine.SpringArmComponent|SetTargetArmLength _springarm (Math|Float|Lerp (Variables|/Script/Engine.SpringArmComponent|GetTargetArmLength _springarm) (Variables|Camera|GetTargetLength) 0.08)))

(event EventBeginPlay
  (Variables|Camera|SetTargetToPan (Transformation|GetWorldLocation (Variables|Default|GetDefaultSceneRoot)))
  (Variables|Camera|SetTargetLength (Variables|/Script/Engine.SpringArmComponent|GetTargetArmLength (Variables|Default|GetSpringArm))))

(event Input|AxisEvents|InputAxisPanHorizontal
  (params (AxisValue :type Float%20%28single-precision%29))
  (Variables|Camera|SetTargetToPan (Math|Vector|MakeVector (.x (Variables|Camera|GetTargetToPan)) (+ (.y (Variables|Camera|GetTargetToPan)) (* AxisValue (Variables|Settings|GetPanSpeed))) (.z (Variables|Camera|GetTargetToPan)))))

(event Input|AxisEvents|InputAxisPanVertical
  (params (AxisValue :type Float%20%28single-precision%29))
  (Variables|Camera|SetTargetToPan (Math|Vector|MakeVector (+ (* AxisValue (Variables|Settings|GetPanSpeed)) (.x (Variables|Camera|GetTargetToPan))) (.y (Variables|Camera|GetTargetToPan)) (.z (Variables|Camera|GetTargetToPan)))))

(event Input|AxisEvents|InputAxisZoom
  (params (AxisValue :type Float%20%28single-precision%29))
  (Variables|Camera|SetTargetLength (Math|Float|Clamp(Float) (+ (* AxisValue (Variables|Settings|GetZoomSpeed)) (Variables|Camera|GetTargetLength)) (Variables|Settings|GetMinZoom) (Variables|Settings|GetMaxZoom))))

(fn ConstructionScript)